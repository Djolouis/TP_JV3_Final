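; BP_NDI_Camera streams a scene capture component's view out through an NDI media output.
; On BeginPlay it points SceneComponentNdi at RenderTarget, creates a media capture from NDIOutput and starts capturing that render target, printing whether this succeeded.
; On EndPlay it stops the active capture if it is still valid.
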(event EventBeginPlay
  (Variables|/Script/Engine.SceneCaptureComponent2D|SetTextureTarget (Variables|Default|GetSceneComponent_Ndi) (Variables|Default|GetRenderTarget))
  (bind _returnvalue (Class|MediaOutput|CreateMediaCapture (Variables|Default|GetNDI_Output)))
  (Variables|Default|SetMediaCaptureActive _returnvalue)
  (bind _returnvalue_2 (Class|MediaCapture|CaptureTextureRenderTarget2D (Variables|Default|GetMediaCaptureActive) (Variables|Default|GetRenderTarget)))
  (if _returnvalue_2
    (Development|PrintString "actif")
    (else
      (Development|PrintString "erreur"))))

(event EventEndPlay
  (params (EndPlayReason :type EEndPlayReason%20Enum :default "Destroyed"))
  (bind _mediacaptureactive (Variables|Default|GetMediaCaptureActive))
  (Utilities|IsValid _mediacaptureactive
    (:Is%20Valid
      (Class|MediaCapture|StopCapture _mediacaptureactive false))))

(fn ConstructionScript)