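; Zombie NPC Blueprint that chases the player and deals melee damage until killed by the player's gun.
; After an opening bite montage, an AIMoveTo loop closes in and plays attack montages, gated by CanAttack.
; The attack's anim notify fires a forward sphere trace that reduces player health; a dead player triggers a one-time bite montage instead.
; GunInteract marks the zombie dead, disables movement and capsule collision, and ragdolls the mesh.
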(event EventBeginPlay
  (bind _returnvalue (Transformation|GetActorLocation))
  (Animation|Montage|PlayMontage (Variables|Character|GetMesh) "/Game/Project/Blueprints/Characters/NPCs/Zombies/Zombie_Quatre/Animations/zom_9Biting_1_Montage.zom_9Biting_1_Montage"
    (:OnCompleted
      ;[0.15 0.15 0.15 0.5] pour que le zombie suive le joueur quand il le voit et l'attaque une fois proche
      ;;[0.15 0.15 0.15 0.5] référence au joueur pour pouvoir lui enlever de la vie
      (bind _asbp_shooter_character (Utilities|Casting|CastToBP_ShooterCharacter (Game|GetPlayerCharacter 0)))
      (bind _output_get (Variables|Default|SetPlayerRef _asbp_shooter_character))
      (if (Variables|Default|GetCanAttack?) :!label _label
        (if (not (Variables|Default|GetZombieDead?))
          (AI|AIMoveTo self "0, 0, 0" _output_get 105.0 false
            (:OnSuccess
              (if (Variables|/Game/Project/Blueprints/Characters/Player/BP_ShooterCharacter.BP_ShooterCharacter_C|GetPlayerDead (Variables|Default|GetPlayerRef))
                (Variables|Default|SetCanAttack? false)
                ;;[0.15 0.15 0.15 0.5] animation quand le zombie tue le joueur
                (Utilities|FlowControl|DoOnce false
                  (:Completed
                    (Animation|Montage|PlayMontage (Variables|Character|GetMesh) "/Game/Project/Blueprints/Characters/NPCs/Zombies/Zombie_Quatre/Animations/zom_9Biting_1_Montage.zom_9Biting_1_Montage")))
                (elif (Variables|Default|GetCanAttack?)
                  (Animation|Montage|PlayMontage (Variables|Character|GetMesh) "/Game/Project/Blueprints/Characters/NPCs/Zombies/Zombie_Quatre/Animations/zom_9Attack_Montage.zom_9Attack_Montage"
                    (:then
                      ;;[0.15 0.15 0.15 0.5] permet d'éviter un problème d'animation qui joue en boucle
                      (Variables|Default|SetCanAttack? false))
                    (:OnCompleted
                      (Variables|Default|SetCanAttack? true :!label _label_2)
                      (goto _label))
                    (:OnInterrupted
                      (goto _label_2))
                    (:OnNotifyBegin
                      ;[0.15 0.15 0.15 0.5] système d'interaction du zombie pour enlever de la vie au joueur lorsqu'il le frappe (lié à un "animNotify" dans le montage de l'animation d'attaque)
                      (bind _returnvalue_2 (Collision|SphereTraceForObjects _returnvalue (+ _returnvalue (* (Math|Vector|GetForwardVector (Transformation|GetActorRotation)) 1e+02)) 2e+01 (Utilities|Array|MakeArray "ObjectTypeQuery3") false 0 "ForDuration" true "(R=1.000000,G=0.000000,B=0.000000,A=1.000000)" "(R=0.000000,G=1.000000,B=0.000000,A=1.000000)" 0.5))
                      (if (not (Variables|Default|GetZombieDead?))
                        (if _returnvalue_2
                          (Default|LessHealth (Variables|/Game/Project/Blueprints/Characters/Player/BP_ShooterCharacter.BP_ShooterCharacter_C|GetBPC_HealthSystem (Variables|Default|GetPlayerRef)) 1e+01))))))))
            (:OnFail
              (goto _label))))))))

(event EventGunInteract
  (bind _mesh (Variables|Character|GetMesh))
  ;[0.15 0.15 0.15 0.5] code lié au gun du joueur pour la mort du zombie
  (Variables|Default|SetZombieDead? true)
  (Pawn|Components|CharacterMovement|DisableMovement (Variables|Character|GetCharacterMovement))
  (Collision|SetCollisionEnabled (Variables|Collision|GetCapsuleComponent) "NoCollision")
  (Collision|SetCollisionEnabled _mesh "QueryAndPhysics")
  (Physics|SetSimulatePhysics _mesh true))

(fn ConstructionScript)