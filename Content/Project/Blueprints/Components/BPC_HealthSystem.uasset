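; BPC_HealthSystem is a component that tracks the player's health and handles healing and damage.
; MoreHealth adds to Health within a fixed clamped range, while LessHealth subtracts damage without clamping.
; Both call the UpdateHealth event dispatcher, and LessHealth also calls PlayerDead whenever Health is at or below zero.
; The event graph holds no active logic, so changes happen only through these two functions.
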(event EventBeginPlay)

(event EventTick
  (params (DeltaSeconds :type Float%20%28single-precision%29)))

(fn MoreHealth
  (params (Amount :type Float%20%28double-precision%29))
  (Variables|Default|SetHealth (Math|Float|Clamp(Float) (+ (Variables|Default|GetHealth) Amount) 0.0 1e+02))
  (Default|CallUpdateHealth))

(fn LessHealth
  (params (Damage :type Float%20%28double-precision%29))
  ;[0.15 0.15 0.15 0.5] on enlève le dommage fait au point de vie du joueur
  (Variables|Default|SetHealth (- (Variables|Default|GetHealth) Damage))
  (Default|CallUpdateHealth)
  (if (<= (Variables|Default|GetHealth) 0.0)
    (Default|CallPlayerDead)))