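; BP_Chrono is a countdown timer that shows the remaining time on its TexteChrono text.
; Every Tick calls a countdown event that subtracts world delta seconds from Temps and clamps it so it never drops below zero.
; The same event splits Temps into floored minutes and seconds and writes them as minutes:seconds, without zero padding.
; Nothing fires when the time runs out, and the construction script is empty.
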(event Custom|Event_timerCounthdown
  (bind _output_get (Variables|Default|SetTemps (Math|Float|Clamp(Float) (- (Variables|Default|GetTemps) (Utilities|Time|GetWorldDeltaSeconds)) 0.0 (Variables|Default|GetTemps))))
  (Rendering|Components|TextRender|SetText (Variables|Default|GetTexte_Chrono) (Utilities|Text|FormatText "{Minutes}:{Secondes}" (Math|Conversions|ToFloat(Integer) (Math|Float|Floor (/ _output_get 6e+01))) (Math|Conversions|ToFloat(Integer) (Math|Float|Floor (Math|Float|%(Float) _output_get 6e+01))))))

(event EventTick
  (params (DeltaSeconds :type Float%20%28single-precision%29))
  (CallFunction|EventTimerCounthdown))

(fn ConstructionScript)